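; Actor component that provides enemy lock-on targeting for its owning character, with functions to find, lock, cycle and reset targets.
; FindAllTarget sphere-traces around the owner for pawns tagged Enemy, and LockOnToTarget sweeps along the camera's forward vector to pick the closest of them.
; ChangeTarget cycles that list by index, toggling indicators through messages.
; Lock and reset changes fire dispatchers, and both traces draw debug shapes.
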(fn FindAllTarget
  (bind _returnvalue (Components|GetOwner))
  (bind _returnvalue_2 (Transformation|GetActorLocation _returnvalue))
  (bind _outhits (Collision|MultiSphereTraceForObjects _returnvalue_2 _returnvalue_2 (Variables|Default|GetTraceDistance) (Utilities|Array|MakeArray "ObjectTypeQuery3") false (Utilities|Array|MakeArray (Components|GetOwner)) "ForDuration" true "(R=1.000000,G=0.000000,B=0.000000,A=1.000000)" "(R=0.000000,G=1.000000,B=0.000000,A=1.000000)" 1.0))
  (for _array_element _outhits
    (if (Actor|ActorHasTag (.HitActor (Collision|BreakHitResult _array_element)) "Enemy")
      (Utilities|Array|AddUnique (Variables|Default|GetTargetEnemy) (.HitActor (Collision|BreakHitResult _array_element)))))
  (return (Variables|Default|GetTargetEnemy)))

(fn Initialize
  (bind _returnvalue (Components|GetOwner))
  (bind _as캐릭터 (Utilities|Casting|CastToCharacter _returnvalue))
  (Variables|Reference|SetCharacter _as캐릭터)
  (bind _camera (Class|BPIThridPersonCharacter|GetCamera(Message) _returnvalue))
  (Variables|Reference|SetCamera _camera))

(fn LockontoTarget
  (bind _camera (Variables|Reference|GetCamera))
  (bind _returnvalue (Transformation|GetWorldLocation _camera))
  (Variables|Default|SetLockedOnTarget 0)
  (Utilities|IsValid (Variables|Default|GetLockedOnTarget)
    (:Is%20Not%20Valid
      (Variables|Default|SetClosetDistance (Variables|Default|GetTraceDistance))
      (bind _outhits (Collision|MultiSphereTraceForObjects _returnvalue (+ _returnvalue (* (Math|Vector|GetForwardVector _camera) (Variables|Default|GetTraceDistance))) (Variables|Default|GetRadiusToLockOn) (Utilities|Array|MakeArray "ObjectTypeQuery3") false 0 "ForDuration" true "(R=0.000000,G=0.923156,B=1.000000,A=1.000000)" "(R=0.095427,G=0.000000,B=1.000000,A=1.000000)" 2.0))
      (for _array_element _outhits
        (if (Utilities|Array|ContainsItem (Variables|Default|GetTargetEnemy) (.HitActor (Collision|BreakHitResult _array_element)))
          (if (< (Transformation|GetDistanceTo (.HitActor (Collision|BreakHitResult _array_element)) (Components|GetOwner)) (Variables|Default|GetClosetDistance))
            (Variables|Default|SetClosetDistance (Transformation|GetDistanceTo (.HitActor (Collision|BreakHitResult _array_element)) (Components|GetOwner)))
            (Variables|Default|SetLockedOnTarget (.HitActor (Collision|BreakHitResult _array_element))))))
      (Default|CallOnLockonNewTarget)
      (return (Variables|Default|GetLockedOnTarget)))))

(fn ResetLockedonTarget
  (Utilities|IsValid (Variables|Default|GetLockedOnTarget)
    (:Is%20Valid
      (Class|BPIEnemyBase|SetIndicatorVisibility(Message) (Variables|Default|GetLockedOnTarget) false)
      (Variables|Default|SetLockedOnTarget 0)
      (Utilities|Array|Clear (Variables|Default|GetTargetEnemy))
      (Variables|Default|SetLockOnTargetIndex 0)
      (Default|CallOnResetLockedonTarget))))

(fn ChangeTarget
  (if (and (Utilities|Array|IsValidIndex (Variables|Default|GetTargetEnemy)) (Utilities|IsValid (Variables|Default|GetLockedOnTarget)))
    (if (not (== (Utilities|Array|Length (Variables|Default|GetTargetEnemy)) 1))
      (for _array_element (Variables|Default|GetTargetEnemy)
        (Class|BPIEnemyBase|SetIndicatorVisibility(Message) _array_element false))
      (if (>= (Variables|Default|GetLockOnTargetIndex) (- (Utilities|Array|Length (Variables|Default|GetTargetEnemy)) 1))
        (Variables|Default|SetLockOnTargetIndex 0)
        (else
          (Variables|Default|SetLockOnTargetIndex (+ (Variables|Default|GetLockOnTargetIndex) 1))))
      (bind _output_get (Variables|Default|SetLockedOnTarget (Utilities|Array|Get(acopy) (Variables|Default|GetTargetEnemy) (Variables|Default|GetLockOnTargetIndex))))
      (Class|BPIEnemyBase|SetIndicatorVisibility(Message) _output_get true)
      (Default|CallOnLockonNewTarget))
    (else
      (Development|PrintString "Target Enemies is not Validate"))))