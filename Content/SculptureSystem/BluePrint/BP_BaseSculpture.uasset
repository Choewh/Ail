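; BP_BaseSculpture is a carvable sculpture block built on a DynamicMeshComponent with Geometry Script.
; The construction script rebuilds it as a PN-tessellated cube with complex-as-simple collision.
; DigSculpture places a wide, thin box in a temporary compute mesh, using the local-space location and given rotation, and boolean-subtracts it.
; It then regenerates collision from the cut mesh, self-unions it and releases the compute meshes.
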(event EventBeginPlay)

(event Collision|EventActorBeginOverlap
  (params (OtherActor :type Actor%20Object%20Reference)))

(event EventTick
  (params (DeltaSeconds :type Float%20%28single-precision%29)))

(fn ConstructionScript
  (bind _returnvalue (DynamicMeshComponent|GetDynamicMesh (Variables|DynamicMeshActor|GetDynamicMeshComponent)))
  (bind _output_get (Variables|Default|SetDynamicMesh _returnvalue))
  (DynamicMesh|Reset _output_get)
  (bind _returnvalue_2 (Class|GeometryScriptLibraryMeshPrimitiveFunctions|AppendBox :TargetMesh (Variables|Default|GetDynamicMesh) :DimensionX 2e+02 :DimensionY 2e+02 :DimensionZ 2e+02 :Debug 0))
  (Class|GeometryScriptLibraryMeshSubdivideFunctions|ApplyPNTessellation :TargetMesh _returnvalue_2 :Debug 0)
  (Class|DynamicMeshComponent|SetComplexasSimpleCollisionEnabled (Variables|DynamicMeshActor|GetDynamicMeshComponent) true true))

(fn DigSculpture
  (params (Location :type Vector) (Transform%20Rotation :type Rotator))
  (bind _returnvalue (DynamicMeshActor|AllocateComputeMesh))
  (bind _returnvalue_2 (Class|GeometryScriptLibraryMeshPrimitiveFunctions|AppendBox :TargetMesh _returnvalue :Transform (Math|Transform|MakeTransform (Math|Transform|InverseTransformLocation (Transformation|GetWorldTransform (Variables|DynamicMeshActor|GetDynamicMeshComponent)) Location) Transform%20Rotation "1.000000,1.000000,1.000000") :DimensionX 5e+02 :DimensionY 3e+01 :DimensionZ 5e+02 :Debug 0))
  (bind _returnvalue_3 (DynamicMeshComponent|GetDynamicMesh (Variables|DynamicMeshActor|GetDynamicMeshComponent)))
  (bind _returnvalue_4 (GeometryScript|Booleans|ApplyMeshBoolean :TargetMesh _returnvalue_3 :ToolMesh _returnvalue_2 :Operation "Subtract" :Debug 0))
  (bind _returnvalue_5 (Class|GeometryScriptLibraryCollisionFunctions|SetDynamicMeshCollisionfromMesh :FromDynamicMesh _returnvalue_4 :ToDynamicMeshComponent (Variables|DynamicMeshActor|GetDynamicMeshComponent) :Debug 0))
  (Class|GeometryScriptLibraryMeshBooleanFunctions|ApplyMeshSelfUnion _returnvalue_5 (Utilities|Struct|MakeGeometryScriptMeshSelfUnionOptions true true true 0.01 0.5) 0)
  (DynamicMeshActor|ReleaseAllComputeMeshes))